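; BP_ConeCollisionVol is a Level 2 trigger volume that fails the player for moving through it too fast.
; When BP_FirstPersonCharacter begins overlapping its Box, it compares the character's velocity magnitude to a fixed speed threshold.
; At or above that speed, it pauses the game and shows the BP_WrongMsg_L2 widget with UI-only input and a visible cursor.
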(event `self.Box.OnComponentBeginOverlap`
  (params (OverlappedComponent :type "PrimitiveComponent Object Reference") (OtherActor :type "Actor Object Reference") (OtherComp :type "PrimitiveComponent Object Reference") (OtherBodyIndex :type Integer) (bFromSweep :type Boolean) (SweepResult :type "HitResult Structure (by ref)"))
  (bind _returnvalue (`GameplayStatics.GetPlayerController` 0))
  (bind _asbp_first_person_character (cast `/Game/FirstPerson/Blueprints/BP_FirstPersonCharacter` OtherActor))
  (if (>= (`KismetMathLibrary.VSize` (`self.GetVelocity` _asbp_first_person_character)) 300.0)
    (`GameplayStatics.SetGamePaused` true)
    (bind _returnvalue_2 (`|CreateWidget` "/Game/Blueprints/UI/L2/BP_WrongMsg_L2.BP_WrongMsg_L2_C"))
    (`WidgetBlueprintLibrary.SetInputMode_UIOnlyEx` _returnvalue _returnvalue_2)
    (set `PlayerController.bShowMouseCursor` true _returnvalue)
    (`UserWidget.AddToViewport` _returnvalue_2 0)))

(fn `UserConstructionScript`)