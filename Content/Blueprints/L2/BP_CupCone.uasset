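; BP_CupCone is a cup cone actor that can lift and spawn a ball, working alongside BP_ConeSelector.
; Lift disables cone selection on the selector, raises the cone along Z with a timeline, then snaps it back and re-enables selection.
; SpawnBall adds an instanced static mesh instance, passing the actor's location and rotation as its transform.
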(event `Lift`
  (bind (_initialpos_x _initialpos_y) (`KismetMathLibrary.BreakVector` (`self.initialPos`)))
  (bind _output_get (set `self.initialPos` (`self.K2_GetActorLocation`)))
  (bind _returnvalue (`GameplayStatics.GetActorOfClass` "/Game/Blueprints/L2/BP_ConeSelector.BP_ConeSelector_C"))
  (set `/Game/Blueprints/L2/BP_ConeSelector.canSelectCone` false _returnvalue)
  (bind (_direction _2secs) (`Timeline|LiftTimeline` :!via `PlayFromStart`)
    (:`Update`
      (`self.K2_SetActorLocation` (`KismetMathLibrary.MakeVector` _initialpos_x _initialpos_y (`KismetMathLibrary.Lerp` (.z _output_get) (+ (.z _output_get) 40.0) _2secs))))
    (:`Finished`
      (`self.K2_SetActorLocation` (`self.initialPos`))
      (bind _returnvalue_2 (`GameplayStatics.GetActorOfClass` "/Game/Blueprints/L2/BP_ConeSelector.BP_ConeSelector_C"))
      (set `/Game/Blueprints/L2/BP_ConeSelector.canSelectCone` true _returnvalue_2))))

(event `SpawnBall`
  (bind _returnvalue (`self.GetTransform`))
  (`InstancedStaticMeshComponent.AddInstance` (`self.InstancedStaticMesh`) (`KismetMathLibrary.MakeTransform` (`KismetMathLibrary.MakeVector` (.x (.location _returnvalue)) (.y (.location _returnvalue)) (.z (.location _returnvalue))) (.rotation _returnvalue)) false))

(fn `UserConstructionScript`)