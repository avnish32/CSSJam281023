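; BP_AnswerScreenTrigger_L2 is a trigger actor that opens the Level 2 answer screen when the player walks into it.
; Overlap on its Cube by BP_FirstPersonCharacter looks up BP_ConeSelector and proceeds only if its CanSelectCone flag is true.
; It then pauses the game, adds the BP_AnswerScreen_L2 widget to the viewport and switches to UI-only input with a visible cursor.
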(event `self.Cube.OnComponentBeginOverlap`
  (params (OverlappedComponent :type "PrimitiveComponent Object Reference") (OtherActor :type "Actor Object Reference") (OtherComp :type "PrimitiveComponent Object Reference") (OtherBodyIndex :type Integer) (bFromSweep :type Boolean) (SweepResult :type "HitResult Structure (by ref)"))
  (bind _returnvalue (`GameplayStatics.GetPlayerController` 0))
  (cast `/Game/FirstPerson/Blueprints/BP_FirstPersonCharacter` OtherActor)
  (`KismetSystemLibrary.PrintString` "answer cube overlapped w player")
  (bind _returnvalue_2 (`GameplayStatics.GetActorOfClass` "/Game/Blueprints/L2/BP_ConeSelector.BP_ConeSelector_C"))
  (if (`/Game/Blueprints/L2/BP_ConeSelector.canSelectCone` _returnvalue_2)
    (`GameplayStatics.SetGamePaused` true)
    (bind _returnvalue_3 (`|CreateWidget` "/Game/Blueprints/UI/L2/BP_AnswerScreen_L2.BP_AnswerScreen_L2_C"))
    (`UserWidget.AddToViewport` _returnvalue_3 0)
    (`WidgetBlueprintLibrary.SetInputMode_UIOnlyEx` _returnvalue _returnvalue_3)
    (set `PlayerController.bShowMouseCursor` true _returnvalue)))

(fn `UserConstructionScript`)