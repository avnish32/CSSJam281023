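; Card actor that flips over temporarily, exposing a Flip event to be triggered from outside this graph.
; Flip sets HasBeenFlipped and IsFlipping, then a timeline lerps the actor from its current rotation to a fixed target along the shortest path.
; One second after the timeline finishes, the card snaps to another fixed rotation and clears IsFlipping, while HasBeenFlipped stays set.
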(event `Flip`
  (set `self.hasBeenFlipped` true)
  (set `self.isFlipping` true)
  (bind _output_get (set `self.initialRot` (`self.K2_GetActorRotation`)))
  (bind (_direction _2_secs) (`Timeline|Flip_Timeline` :!via `PlayFromStart`)
    (:`Update`
      (`self.K2_SetActorRotation` (`KismetMathLibrary.RLerp` _output_get (`KismetMathLibrary.MakeRotator` 0.0 0.0 90.0) _2_secs true)))
    (:`Finished`
      (`KismetSystemLibrary.Delay` 1.0)
      (`self.K2_SetActorRotation` (struct :`Yaw` 90.0 :`Roll` 180.0))
      (set `self.isFlipping` false))))

(fn `UserConstructionScript`)